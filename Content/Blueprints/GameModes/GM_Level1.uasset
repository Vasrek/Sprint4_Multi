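; GM_Level1 is the Level 1 game mode that tracks connected players and shares their info across all player controllers.
; It adds controllers to a list on PostLogin and removes them on logout.
; GetAllPlayerInfo appends each incoming player info entry, sends the full list to every PC_Level1, then updates each character's displayed pseudo and formatted health.
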(event `self.K2_PostLogin`
  (params (NewPlayer :type "PlayerController Object Reference"))
  (`KismetArrayLibrary.Array_Add` (`self.AllPlayersControllers`) NewPlayer))

(event `self.K2_OnLogout`
  (params (ExitingController :type "Controller Object Reference"))
  (bind _asplayer_controller (cast `PlayerController` ExitingController))
  (`KismetArrayLibrary.Array_RemoveItem` (`self.AllPlayersControllers`) _asplayer_controller))

(event `GetAllPlayerInfo`
  (params (PlayerInfo :type "/Game/Blueprints/Structures/S_PlayerInfo Structure"))
  (`KismetArrayLibrary.Array_Add` (`self.AllPlayersInfo`) PlayerInfo)
  (for _array_element (`self.AllPlayersControllers`)
    (bind _aspc_level_1 (cast `/Game/Blueprints/PlayerControllers/PC_Level1` _array_element))
    (`/Game/Blueprints/PlayerControllers/PC_Level1.GetAllPlayersInfo` _aspc_level_1 (`self.AllPlayersInfo`)))
  (for _array_element_2 (`self.AllPlayersInfo`)
    (bind (_pseudo _health _character) (break `/Game/Blueprints/Structures/S_PlayerInfo` _array_element_2))
    (`/Game/Blueprints/Character/BP_MyCharacter.UpdateHealthPseudo` _character _pseudo (`|FormatText` "{health}/100" _health))))

(fn `UserConstructionScript`)