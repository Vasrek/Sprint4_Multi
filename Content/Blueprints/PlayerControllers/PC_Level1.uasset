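; Player controller for Level 1 that tracks its player's info (name, health, character) in a multiplayer test setup.
; On BeginPlay it fills a PlayerInfo struct with a random name, max health and the possessed character, then sends it to GM_Level1.
; GetAllPlayersInfo prints every player's health from a received list.
; Debug keys lower health and resend it (K), or attempt joining a localhost server (O).
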(event `self.ReceiveBeginPlay`
  (`self.GetPlayerCharacterReference`))

(event `GetPlayerCharacterReference`
  (bind _asbp_my_character (cast `/Game/Blueprints/Character/BP_MyCharacter` (`self.K2_GetPawn`)))
  (bind _structout (setmembers `/Game/Blueprints/Structures/S_PlayerInfo` :`StructRef` (`self.PlayerInfo`) :`Pseudo` (`|FormatText` "Player{X}" (`KismetMathLibrary.RandomIntegerInRange` 1 100)) :`health` (`self.MaxHealth`) :`Character` _asbp_my_character))
  (`self.SendPlayerInfoToServer` _structout))

(event `SendPlayerInfoToServer`
  (params (PlayerInfo :type "/Game/Blueprints/Structures/S_PlayerInfo Structure"))
  (`/Game/Blueprints/GameModes/GM_Level1.GetAllPlayerInfo` (cast `/Game/Blueprints/GameModes/GM_Level1` (`GameplayStatics.GetGameMode`) :!pure true) PlayerInfo))

(event `Key|K`
  (params (Key :type "Key Structure"))
  (bind _playerinfo (`self.PlayerInfo`))
  (:`Pressed`
    (bind _structout (setmembers `/Game/Blueprints/Structures/S_PlayerInfo` :`StructRef` _playerinfo :`health` (- (`.health_8_AC095FA2404529FC2B845F8CFCD3BE0B` (break `/Game/Blueprints/Structures/S_PlayerInfo` _playerinfo)) 20)))
    (`self.SendPlayerInfoToServer` _structout)
    (bind (_pseudo _health) (break `/Game/Blueprints/Structures/S_PlayerInfo` _structout))
    (`KismetSystemLibrary.PrintString` (`KismetStringLibrary.Concat_StrStr` (`KismetTextLibrary.Conv_TextToString` _pseudo) " health left: " (`KismetStringLibrary.Conv_IntToString` _health)) true true (struct :`R` 0.554167 :`G` 0.38622 :`B` 0.050984 :`A` 1.0) 60.0)))

(event `GetAllPlayersInfo`
  (params (PlayerInfo :type "Array of /Game/Blueprints/Structures/S_PlayerInfo Structure"))
  (for _array_element PlayerInfo
    (bind (_pseudo _health) (break `/Game/Blueprints/Structures/S_PlayerInfo` _array_element))
    (`KismetSystemLibrary.PrintString` (`KismetStringLibrary.Concat_StrStr` (`KismetTextLibrary.Conv_TextToString` _pseudo) " health left: " (`KismetStringLibrary.Conv_IntToString` _health)) true true (struct :`R` 0.7375 :`G` 0.033396 :`A` 1.0) 15.0)))

(event `Key|O`
  (params (Key :type "Key Structure"))
  (:`Pressed`
    (`GameplayStatics.OpenLevel` "open 127.0.0.1:7777")))

(fn `UserConstructionScript`)